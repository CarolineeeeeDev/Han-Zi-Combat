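; EnterGame2BP is a VR actor that switches the player into Game 2 and returns pistols entering its trigger box.
; With input enabled at BeginPlay, the right B button sets InGame2 on the VRPawn and zeroes Game2UpdateScore on the first press only.
; A pistol overlapping Box is destroyed and respawned at a hardcoded transform.
; The overlap's DoOnce resets only after that respawn, so a non-pistol overlap leaves it closed.
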(event OnComponentBeginOverlap(Box)
  (params (OverlappedComponent :type Primitive%20Component%20Object%20Reference) (OtherActor :type Actor%20Object%20Reference) (OtherComp :type Primitive%20Component%20Object%20Reference) (OtherBodyIndex :type Integer) (bFromSweep :type Boolean) (SweepResult :type Hit%20Result%20Structure%20%28by%20ref%29))
  (Utilities|FlowControl|DoOnce false :!label _label
    (:Completed
      (bind _aspistol (Utilities|Casting|CastToPistol OtherActor))
      (Actor|DestroyActor _aspistol)
      (Game|SpawnActorfromClass "/Game/VRTemplate/Blueprints/Pistol.Pistol_C" (Math|Transform|MakeTransform "-150.519058,-455.433167,99.425728" "90.000000, 0,-133.842041" "0.500000,0.500000,0.500000") "Undefined" 0 0)
      (goto _label Reset))))

(event EventBeginPlay
  (Input|EnableInput (Game|GetPlayerController 0)))

(event Collision|EventActorBeginOverlap
  (params (OtherActor :type Actor%20Object%20Reference)))

(event EventTick
  (params (DeltaSeconds :type Float%20%28single-precision%29)))

(event Input|ActionEvents|InputActionPressRightB
  (params (Key :type Key%20Structure :default "None"))
  (:Pressed
    (bind _asvrpawn (Utilities|Casting|CastToVRPawn (Game|Player|GetPlayerPawn 0)))
    (Variables|/Game/VRTemplate/Blueprints/VRPawn.VRPawn_C|SetInGame2 _asvrpawn true)
    (Utilities|FlowControl|DoOnce false
      (:Completed
        (Variables|/Game/VRTemplate/Blueprints/VRPawn.VRPawn_C|SetGame2UpdateScore _asvrpawn 0)))))

(fn ConstructionScript)