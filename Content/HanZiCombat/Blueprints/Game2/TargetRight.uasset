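; Moving "right" target for the VR pawn's second minigame, scored when projectiles hit it.
; While InGame2 is set, a timeline slides the mesh along Y, and its delayed update swaps materials from every other Game2Data row, destroying the actor when rows run out.
; A DoOnce, reset per row, allows one hit, which plays a sound and raises or lowers the pawn's score by the row's Correct flag, tracking the best.
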(event OnComponentBeginOverlap(StaticMesh)
  (params (OverlappedComponent :type Primitive%20Component%20Object%20Reference) (OtherActor :type Actor%20Object%20Reference) (OtherComp :type Primitive%20Component%20Object%20Reference) (OtherBodyIndex :type Integer) (bFromSweep :type Boolean) (SweepResult :type Hit%20Result%20Structure%20%28by%20ref%29))
  (Utilities|Casting|CastToProjectile OtherActor)
  (bind _returnvalue (Utilities|GetDataTableRow "/Game/HanZiCombat/Data/Game2Data.Game2Data" (Utilities|String|StringToName (Utilities|String|ToString(Integer) (- (Variables|Default|GetIndex) 2))))
    (:then
      (Utilities|FlowControl|DoOnce false
        (:Completed
          (if (.Correct (Utilities|Struct|BreakGame2Struct _returnvalue))
            (Audio|PlaySound2D "/Engine/VREditor/Sounds/UI/Camera_Shutter.Camera_Shutter" 1.0 1.0 0.0 0 0)
            (bind _asvrpawn (Utilities|Casting|CastToVRPawn (Game|Player|GetPlayerPawn 0)))
            (bind _output_get (Variables|/Game/VRTemplate/Blueprints/VRPawn.VRPawn_C|SetGame2UpdateScore _asvrpawn (+ (Variables|/Game/VRTemplate/Blueprints/VRPawn.VRPawn_C|GetGame2UpdateScore _asvrpawn) 10)))
            (if (> _output_get (Variables|/Game/VRTemplate/Blueprints/VRPawn.VRPawn_C|GetGame2Score _asvrpawn))
              (bind _output_get_2 (Variables|/Game/VRTemplate/Blueprints/VRPawn.VRPawn_C|SetGame2Score _asvrpawn _output_get))
              (Development|PrintString (Utilities|String|ToString(Integer) _output_get_2)))
            (else
              (Audio|PlaySound2D "/Engine/EditorSounds/Notifications/CompileFailed_Cue.CompileFailed_Cue" 1.0 1.0 0.0 0 0)
              (bind _asvrpawn_2 (Utilities|Casting|CastToVRPawn (Game|Player|GetPlayerPawn 0)))
              (Variables|/Game/VRTemplate/Blueprints/VRPawn.VRPawn_C|SetGame2UpdateScore _asvrpawn_2 (- (Variables|/Game/VRTemplate/Blueprints/VRPawn.VRPawn_C|GetGame2UpdateScore _asvrpawn_2) 5)))))))))

(event EventTick
  (params (DeltaSeconds :type Float%20%28single-precision%29))
  (bind _staticmesh (Variables|Default|GetStaticMesh))
  (bind _asvrpawn (Utilities|Casting|CastToVRPawn (Game|Player|GetPlayerPawn 0)))
  (if (Variables|/Game/VRTemplate/Blueprints/VRPawn.VRPawn_C|GetInGame2 _asvrpawn)
    (Utilities|FlowControl|DoOnce false
      (:Completed
        (Rendering|Material|SetMaterial (Variables|Default|GetStaticMesh) 0 "/Game/HanZiCombat/Materials/Game2Material/Target/Dan2Material.Dan2Material")
        (bind _newtrack_0 (Timeline|Timeline_0 Play)
          (:Update
            (Transformation|SetRelativeLocation _staticmesh (Math|Vector|MakeVector 0.0 (Math|Float|Lerp 0.0 1.2e+03 _newtrack_0) 0.0) false false)
            (Utilities|FlowControl|Delay 5.0)
            (bind _returnvalue (Utilities|GetDataTableRow "/Game/HanZiCombat/Data/Game2Data.Game2Data" (Utilities|String|StringToName (Utilities|String|ToString(Integer) (Variables|Default|GetIndex))))
              (:then
                (Rendering|Material|SetMaterial _staticmesh 0 (.Material (Utilities|Struct|BreakGame2Struct _returnvalue)))
                (Variables|Default|SetIndex (+ (Variables|Default|GetIndex) 2))
                (Utilities|FlowControl|DoOnce false) ; enters at Reset
              )
              (:RowNotFound
                (Actor|DestroyActor)))))))
    (else
      (Timeline|Timeline_0 Stop))))

(fn ConstructionScript)