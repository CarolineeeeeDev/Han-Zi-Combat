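; Moving target cube for Game1 of the VR HanZi combat game, scored when struck by a LightSaber.
; On BeginPlay a Timeline slides its scaled-up mesh along relative Y.
; A saber overlap looks up the cube's Index row in Game1Data once, then plays a right or wrong sound and destroys the cube.
; Correct hits add points on VRPawn and raise Game1Score when exceeded, while wrong hits subtract points.
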(event OnComponentBeginOverlap(StaticMesh)
  (params (OverlappedComponent :type Primitive%20Component%20Object%20Reference) (OtherActor :type Actor%20Object%20Reference) (OtherComp :type Primitive%20Component%20Object%20Reference) (OtherBodyIndex :type Integer) (bFromSweep :type Boolean) (SweepResult :type Hit%20Result%20Structure%20%28by%20ref%29))
  (Utilities|Casting|CastToLightSaber OtherActor)
  (bind _returnvalue (Utilities|GetDataTableRow "/Game/HanZiCombat/Data/Game1Data.Game1Data" (Utilities|String|StringToName (Utilities|String|ToString(Integer) (Variables|Default|GetIndex))))
    (:then
      (Utilities|FlowControl|DoOnce false
        (:Completed
          (if (.Correct (Utilities|Struct|BreakGame1Struct _returnvalue))
            (Audio|PlaySound2D "/Engine/VREditor/Sounds/UI/Camera_Shutter.Camera_Shutter" 1.0 1.0 0.0 0 0)
            (bind _asvrpawn (Utilities|Casting|CastToVRPawn (Game|Player|GetPlayerPawn 0)))
            (bind _output_get (Variables|/Game/VRTemplate/Blueprints/VRPawn.VRPawn_C|SetGame1UpdateScore _asvrpawn (+ (Variables|/Game/VRTemplate/Blueprints/VRPawn.VRPawn_C|GetGame1UpdateScore _asvrpawn) 10)))
            (if (> _output_get (Variables|/Game/VRTemplate/Blueprints/VRPawn.VRPawn_C|GetGame1Score _asvrpawn))
              (Variables|/Game/VRTemplate/Blueprints/VRPawn.VRPawn_C|SetGame1Score _asvrpawn _output_get))
            (Actor|DestroyActor)
            (else
              (Audio|PlaySound2D "/Engine/EditorSounds/Notifications/CompileFailed.CompileFailed" 1.0 1.0 0.0 0 0)
              (bind _asvrpawn_2 (Utilities|Casting|CastToVRPawn (Game|Player|GetPlayerPawn 0)))
              (Variables|/Game/VRTemplate/Blueprints/VRPawn.VRPawn_C|SetGame1UpdateScore _asvrpawn_2 (- (Variables|/Game/VRTemplate/Blueprints/VRPawn.VRPawn_C|GetGame1UpdateScore _asvrpawn_2) 5))
              (Actor|DestroyActor))))))))

(event EventBeginPlay
  (bind _newtrack_0 (Timeline|Timeline_0 Play)
    (:Update
      (Transformation|SetRelativeTransform (Variables|Default|GetStaticMesh) (Math|Transform|MakeTransform (Math|Vector|MakeVector 0.0 (Math|Float|Lerp 0.0 2e+03 _newtrack_0) 0.0) "0, 0, 0" "5.000000,5.000000,5.000000") false false))))

(event Collision|EventActorBeginOverlap
  (params (OtherActor :type Actor%20Object%20Reference)))

(event EventTick
  (params (DeltaSeconds :type Float%20%28single-precision%29)))

(fn ConstructionScript)