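; Spawner actor for Game 1: creates the question actor, resets the VR pawn's score and emits the moving cubes.
; Once InGame1 is true, a one-shot Tick trigger starts a delayed loop through Game1Data rows by index.
; Each row spawns a MoveCubeBP at random Y/Z with that row's material and index.
; When rows run out, it spawns Game1RestartBP, clears InGame1 and destroys the LightSabers, question and itself.
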(event Collision|EventActorBeginOverlap
  (params (OtherActor :type Actor%20Object%20Reference)))

(event EventBeginPlay
  (bind _asvrpawn (Utilities|Casting|CastToVRPawn (Game|Player|GetPlayerPawn 0)))
  (Variables|/Game/VRTemplate/Blueprints/VRPawn.VRPawn_C|SetGame1UpdateScore _asvrpawn 0)
  (bind _returnvalue (Game|SpawnActorfromClass "/Game/HanZiCombat/Blueprints/Game1/Game1QuestionBP.Game1QuestionBP_C" (Math|Transform|MakeTransform "1645.952881,77.809204,264.781677" "0,180.000000, 0" "0.500000,0.500000,0.500000") "Undefined" 0 0))
  (Variables|Default|SetQuestion _returnvalue))

(event EventTick
  (params (DeltaSeconds :type Float%20%28single-precision%29))
  (bind _question (Variables|Default|GetQuestion))
  (bind _asvrpawn (Utilities|Casting|CastToVRPawn (Game|Player|GetPlayerPawn 0)))
  (if (Variables|/Game/VRTemplate/Blueprints/VRPawn.VRPawn_C|GetInGame1 _asvrpawn)
    (Utilities|FlowControl|DoOnce false
      (:Completed
        (bind _returnvalue (Utilities|GetDataTableRow "/Game/HanZiCombat/Data/Game1Data.Game1Data" (Utilities|String|StringToName (Utilities|String|ToString(Integer) (Variables|Default|GetIndex))) :!label _label)
          (:then
            (bind _returnvalue_2 (Game|SpawnActorfromClass "/Game/HanZiCombat/Blueprints/Game1/MoveCubeBP.MoveCubeBP_C" (Math|Transform|MakeTransform (Math|Vector|MakeVector (Math|Float|Absolute(Float) 1747.844238) (Math|Random|RandomFloatinRange -47.638885 401.751465) (Math|Random|RandomFloatinRange 67.438095 414.021301)) "0,90.000000, 0") "Undefined" 0 0))
            (Variables|/Game/HanZiCombat/Blueprints/Game1/MoveCubeBP.MoveCubeBP_C|SetIndex _returnvalue_2 (Variables|Default|GetIndex))
            (Rendering|Material|SetMaterial (Variables|/Game/HanZiCombat/Blueprints/Game1/MoveCubeBP.MoveCubeBP_C|GetStaticMesh _returnvalue_2) 0 (.Material (Utilities|Struct|BreakGame1Struct _returnvalue)))
            (Utilities|FlowControl|Delay 3.0)
            (Variables|Default|SetIndex (+ (Variables|Default|GetIndex) 1))
            (goto _label))
          (:RowNotFound
            (Game|SpawnActorfromClass "/Game/HanZiCombat/Blueprints/Game1/Game1RestartBP.Game1RestartBP_C" (Math|Transform|MakeTransform "171.229233,15.233612,141.817032" "0,90.000000, 0" "0.500000,0.500000,0.500000") "Undefined" 0 0)
            (bind _asvrpawn_2 (Utilities|Casting|CastToVRPawn (Game|Player|GetPlayerPawn 0)))
            (Variables|/Game/VRTemplate/Blueprints/VRPawn.VRPawn_C|SetInGame1 _asvrpawn_2 false)
            (bind _outactors (Actor|GetAllActorsOfClass "/Game/HanZiCombat/Blueprints/Game1/LightSaber.LightSaber_C"))
            (for _array_element _outactors
              (Utilities|IsValid _array_element
                (:Is%20Valid
                  (Actor|DestroyActor _array_element)
                  (Utilities|IsValid _question
                    (:Is%20Valid
                      (Actor|DestroyActor _question)
                      (Actor|DestroyActor))))))))))))

(fn ConstructionScript)