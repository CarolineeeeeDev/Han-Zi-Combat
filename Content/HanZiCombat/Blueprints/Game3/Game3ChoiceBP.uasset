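; Game 3 choice actor that runs a timed true/false quiz for the VR pawn, using green and red buttons.
; Tick, gated by a DoOnce, reads each QuestionData row by index and briefly enables input until rows run out.
; Right and left triggers animate their button via timelines and set a temporary answer.
; The answer is scored with a sound, updating the pawn's running and best scores before resetting for the next question.
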(event Collision|EventActorBeginOverlap
  (params (OtherActor :type Actor%20Object%20Reference)))

(event EventTick
  (params (DeltaSeconds :type Float%20%28single-precision%29))
  (bind _returnvalue (Game|GetPlayerController 0))
  (bind _asvrpawn (Utilities|Casting|CastToVRPawn (Game|Player|GetPlayerPawn 0)))
  (if (Variables|/Game/VRTemplate/Blueprints/VRPawn.VRPawn_C|GetInGame3 _asvrpawn)
    (Utilities|FlowControl|DoOnce false :!label _label
      (:Completed
        (bind _returnvalue_2 (Utilities|GetDataTableRow "/Game/HanZiCombat/Data/QuestionData.QuestionData" (Utilities|String|StringToName (Utilities|String|ToString(Integer) (Variables|Default|GetIndex))))
          (:then
            (Input|EnableInput _returnvalue)
            (Utilities|FlowControl|Delay 3.0)
            (Input|DisableInput _returnvalue)
            (bind _asvrpawn_2 (Utilities|Casting|CastToVRPawn (Game|Player|GetPlayerPawn 0)))
            (if (.Answer (Utilities|Struct|BreakQuestionStructure _returnvalue_2))
              (if (== (Variables|Default|GetAnswer) 2)
                _
                (else
                  (Variables|/Game/VRTemplate/Blueprints/VRPawn.VRPawn_C|SetGame3UpdateScore _asvrpawn_2 (- (Variables|/Game/VRTemplate/Blueprints/VRPawn.VRPawn_C|GetGame3UpdateScore _asvrpawn_2) 5) :!label _label_2)
                  (Audio|PlaySound2D "/Engine/EditorSounds/Notifications/CompileFailed.CompileFailed" 1.0 1.0 0.0 0 0)
                  (Utilities|FlowControl|Delay 2.0)
                  (Variables|Default|SetIndex (+ (Variables|Default|GetIndex) 1))
                  (goto _label Reset)))
              (elif (== (Variables|Default|GetAnswer) 1)
                _
                (else
                  (goto _label_2))))
            (bind _output_get (Variables|/Game/VRTemplate/Blueprints/VRPawn.VRPawn_C|SetGame3UpdateScore _asvrpawn_2 (+ (Variables|/Game/VRTemplate/Blueprints/VRPawn.VRPawn_C|GetGame3UpdateScore _asvrpawn_2) 10)))
            (Audio|PlaySound2D "/Engine/VREditor/Sounds/UI/Camera_Shutter.Camera_Shutter" 1.0 1.0 0.0 0 0)
            (Utilities|FlowControl|Delay 2.0)
            (Variables|Default|SetIndex (+ (Variables|Default|GetIndex) 1))
            (if (> _output_get (Variables|/Game/VRTemplate/Blueprints/VRPawn.VRPawn_C|GetGame3Score _asvrpawn_2))
              (Variables|/Game/VRTemplate/Blueprints/VRPawn.VRPawn_C|SetGame3Score _asvrpawn_2 _output_get)
              (goto _label Reset)
              (else
                (goto _label Reset))))
          (:RowNotFound
            (Input|DisableInput (Game|GetPlayerController 0))))))))

(event Input|ActionEvents|InputActionTriggerRight
  (params (Key :type Key%20Structure :default "None"))
  (:Pressed
    (bind _newtrack_0 (Timeline|Timeline_0 PlayFromStart)
      (:Update
        (Transformation|SetRelativeLocation (Variables|Default|GetSceneGreen) (Math|Vector|MakeVector 36.690662 21.688244 (Math|Float|Lerp 95.80645 85.80645 _newtrack_0)) false false)
        (Variables|Default|SetAnswer 2)
        (Utilities|FlowControl|Delay 3.0)
        (Variables|Default|SetAnswer 0)))))

(event Input|ActionEvents|InputActionTriggerLeft
  (params (Key :type Key%20Structure :default "None"))
  (:Pressed
    (bind _newtrack_0 (Timeline|Timeline_1 PlayFromStart)
      (:Update
        (Transformation|SetRelativeLocation (Variables|Default|GetSceneRed) (Math|Vector|MakeVector -34.582901 0.0 (Math|Float|Lerp 95.80645 85.80645 _newtrack_0)) false false)
        (Variables|Default|SetAnswer 1)
        (Utilities|FlowControl|Delay 3.0)
        (Variables|Default|SetAnswer 0)))))

(fn ConstructionScript)