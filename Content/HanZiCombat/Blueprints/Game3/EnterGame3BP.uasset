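; EnterGame3BP is the entry actor that sets up and starts Game 3 for the VR player.
; On BeginPlay it enables player input, destroys any Game3RestartBP actors and spawns a Game3ChoiceBP at a fixed transform.
; Each PressRightB press sets InGame3 on the VRPawn.
; A DoOnce lets only the first press reset the pawn's Game 3 score and spawn the Game3QuestionBP, keeping a reference to it.
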(event Collision|EventActorBeginOverlap
  (params (OtherActor :type Actor%20Object%20Reference)))

(event EventTick
  (params (DeltaSeconds :type Float%20%28single-precision%29)))

(event EventBeginPlay
  (Utilities|FlowControl|Sequence
    (:then_0
      (Input|EnableInput (Game|GetPlayerController 0))
      (bind _outactors (Actor|GetAllActorsOfClass "/Game/HanZiCombat/Blueprints/Game3/Game3RestartBP.Game3RestartBP_C"))
      (for _array_element _outactors
        (Utilities|IsValid _array_element
          (:Is%20Valid
            (Actor|DestroyActor _array_element)))))
    (:then_1
      (Game|SpawnActorfromClass "/Game/HanZiCombat/Blueprints/Game3/Game3ChoiceBP.Game3ChoiceBP_C" (Math|Transform|MakeTransform "87.648575,0.810788,0.000504" "0,90.000000, 0") "Undefined" 0 0))))

(event Input|ActionEvents|InputActionPressRightB
  (params (Key :type Key%20Structure :default "None"))
  (:Pressed
    (bind _asvrpawn (Utilities|Casting|CastToVRPawn (Game|Player|GetPlayerPawn 0)))
    (Variables|/Game/VRTemplate/Blueprints/VRPawn.VRPawn_C|SetInGame3 _asvrpawn true)
    (Utilities|FlowControl|DoOnce false
      (:Completed
        (Variables|/Game/VRTemplate/Blueprints/VRPawn.VRPawn_C|SetGame3UpdateScore _asvrpawn 0)
        (bind _returnvalue (Game|SpawnActorfromClass "/Game/HanZiCombat/Blueprints/Game3/Game3QuestionBP.Game3QuestionBP_C" (Math|Transform|MakeTransform "1295.306396,14.093594,157.429764" "0,180.000000, 0" "0.600000,0.600000,0.600000") "Undefined" 0 0))
        (Variables|Default|SetQuestion _returnvalue)))))

(fn ConstructionScript)